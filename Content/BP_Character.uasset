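; Character that exercises an Inventory component through number-key debug inputs for adding, removing, dropping, transferring and printing items.
; Adds use random health or mana potions from the item database, directly or via a spawned BaseItem, with one granted on locally controlled BeginPlay.
; Transfers target the first other BP_Character.
; For TransferItemToInventory, local control caches that character's item IDs on one press, then transfers a random one on the next.
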(event `Retrieve Inventory Items`
  (params (Character :type "/Game/BP_Character Object Reference"))
  (bind _returnvalue (`InventoryComponent.GetInventoryList` (`/Game/BP_Character.Inventory` Character) "Inv_Item"))
  (bind _keys (`BlueprintMapLibrary.Map_Keys` _returnvalue))
  (`self.Save Inventory Items` _keys))

(event `self.ReceiveBeginPlay`
  (if (`self.IsLocallyControlled`)
    (`self.AddItem`)))

(event `Save Inventory Items`
  (params (`Inventory Items` :type "Array of Guid Structure"))
  (bind _output_get (set `self.OtherInventoryItems` `Inventory Items`))
  (for _array_element _output_get
    (`KismetSystemLibrary.PrintString` (`KismetGuidLibrary.Conv_GuidToString` _array_element))))

(event `Key|Five`
  (params (Key :type "Key Structure"))
  ;[0 1 0.313] Transferring
  (:`Pressed`
    (`self.TransferItemFromInventory` (`self.Find Inventory Character`))))

(event `Key|One`
  (params (Key :type "Key Structure"))
  ;[0 1 0.313] Adding
  (:`Pressed`
    (`self.AddItem`)))

(event `Key|Two`
  (params (Key :type "Key Structure"))
  ;[0 1 0.313] Adding
  (:`Pressed`
    (`self.AddItemFromWorld`)))

(event `Key|Six`
  (params (Key :type "Key Structure"))
  ;[0 1 0.313] Transferring
  (:`Pressed`
    (`self.TransferItemToInventory` (`self.Find Inventory Character`))))

(event `Key|Seven`
  (params (Key :type "Key Structure"))
  ;[0 1 0.313] Printing
  (:`Pressed`
    (`self.PrintInventory`)))

(event `Key|Three`
  (params (Key :type "Key Structure"))
  ;[0 1 0.313] Removing
  (:`Pressed`
    (`self.RemoveItem` "Inv_Item")))

(event `Key|Four`
  (params (Key :type "Key Structure"))
  ;[0 1 0.313] Removing
  (:`Pressed`
    (`self.RemoveItem` "Inv_Item" true)))

(fn `AddItem`
  (bind (_id _sortorder _itemname _displayname _description _interacttext _itemtype) (break `_Item` (`self.CreateRandomInventoryItem`)))
  (`InventoryInterface.TryAddItem` (`self.Inventory`) _itemname null _itemtype))

(fn `AddItemFromWorld`
  (locals (NewLocalVar :type "Guid Structure"))
  (bind _returnvalue (`|SpawnActorFromClass` "/Script/InventorySystem.BaseItem" (`self.GetTransform`) "Undefined" "MultiplyWithRoot" null null))
  (`InventoryItemInterface.SetItem` _returnvalue (`self.CreateRandomInventoryItem`))
  (bind (_returnvalue_id _returnvalue_sortorder _returnvalue_itemname _returnvalue_displayname _returnvalue_description _returnvalue_interacttext _returnvalue_itemtype) (break `_Item` (`InventoryItemInterface.GetItem` _returnvalue)))
  (`InventoryInterface.TryAddItem` (`self.Inventory`) _returnvalue_itemname _returnvalue _returnvalue_itemtype))

(fn `CreateRandomInventoryItem`
  (returns (Item :type "_Item Structure"))
  (locals (ItemId :type Name))
  (if (`KismetMathLibrary.RandomBool`)
    (set `local.ItemId` "HealthPotion")
    (else
      (set `local.ItemId` "ManaPotion")))
  (bind _item (`InventoryInterface.GetDataBaseItem` (`self.Inventory`) (`local.ItemId`)))
  (bind (_id _sortorder _itemname _displayname _description _interacttext _itemtype _image _actualclass _worldclass _globalinformation) (break `_Item` _item))
  (return (make `_Item` (`KismetGuidLibrary.NewGuid`) _sortorder _itemname _displayname _description _interacttext _itemtype _image _actualclass _worldclass _globalinformation)))

(fn `Find Inventory Character`
  (returns (`Other Inventory Character` :type "/Game/BP_Character Object Reference"))
  (bind _outactors (`GameplayStatics.GetAllActorsOfClass` "BP_Character_C"))
  (for _array_element _outactors
    (if (!= _array_element self)
      (bind _output_get (set `self.OtherInventoryCharacter` _array_element))
      (return _output_get))))

(fn `PrintInventory`
  (`InventoryComponent.ListInventory` (`self.Inventory`)))

(fn `RemoveItem`
  (params (Type :type "EItemType Enum" :default "Inv_Item") (SpawnItem :type Boolean))
  (`InventoryInterface.TryRemoveItem` (`self.Inventory`) (`self.ReturnRandomInventoryItemId` Type) Type SpawnItem))

(fn `ReturnRandomInventoryItemId`
  (params (Type :type "EItemType Enum" :default "Inv_Item"))
  (returns (`Item Id` :type "Guid Structure"))
  (locals (`Item Ids` :type "Array of Guid Structure"))
  (bind _returnvalue (`InventoryComponent.GetInventoryList` (`self.Inventory`) Type))
  (bind _keys (`BlueprintMapLibrary.Map_Keys` _returnvalue))
  (return (`KismetArrayLibrary.Array_Random` _keys)))

(fn `TransferItemFromInventory`
  (params (OtherCharacter :type "/Game/BP_Character Object Reference"))
  (locals (ItemIds :type "Array of Guid Structure"))
  (bind _inventory (`/Game/BP_Character.Inventory` OtherCharacter))
  (cast `InventoryInterface` _inventory)
  (`InventoryInterface.TryTransferItem` (`self.Inventory`) (`self.ReturnRandomInventoryItemId` "Inv_Item") _inventory "Inv_Item"))

(fn `TransferItemToInventory`
  (params (OtherCharacter :type "/Game/BP_Character Object Reference"))
  (locals (ItemIds :type "Array of Guid Structure") (`Other Inventory` :type "InventoryComponent Object Reference") (`Item Id` :type "Guid Structure"))
  (bind _inventory (`/Game/BP_Character.Inventory` OtherCharacter))
  (cast `InventoryInterface` _inventory)
  (set `local.Other Inventory` _inventory)
  (set `local.Item Id` (`self.ReturnRandomInventoryItemId` OtherCharacter "Inv_Item"))
  (if (`self.IsLocallyControlled`)
    (if (`KismetArrayLibrary.Array_IsEmpty` (`self.OtherInventoryItems`))
      (`self.Retrieve Inventory Items` (`local.OtherCharacter`))
      (else
        (`InventoryInterface.TryTransferItem` (`self.Inventory`) (`KismetArrayLibrary.Array_Random` (`self.OtherInventoryItems`)) (`local.Other Inventory`) "Inv_Item")
        (`KismetArrayLibrary.Array_Clear` (`self.OtherInventoryItems`))))
    (else
      (`InventoryInterface.TryTransferItem` (`self.Inventory`) (`local.Item Id`) (`local.Other Inventory`) "Inv_Item"))))

(fn `UserConstructionScript`)